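; BP_Cannon is a cannon actor that fires automatically and repeatedly from BeginPlay.
; After a fire-rate delay, it spawns a BP_Projectile at its Arrow component's location and rotation, scaled by ProjectileScale.
; FireTimeline then animates the barrel's relative Y location, and its Cannon Fired event track loops back to the delay, so firing cycles without using Tick.
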(event `self.ReceiveBeginPlay`
  (`KismetSystemLibrary.Delay` (`self.CannonFireRate`) :!label _label)
  (`self.SpawnProjectile`)
  (bind (_direction _barrel_barrel_location) (`Timeline|Fire Timeline` :!via `PlayFromStart`)
    (:`Update`
      (`self.MoveCannonBarrel` _barrel_barrel_location))
    (:`Cannon Fired`
      (goto _label))))

(fn `MoveCannonBarrel`
  (params (CannonBarrelYLocation :type "Float (double-precision)"))
  (`SceneComponent.K2_SetRelativeLocation` (`self.CannonBarrel`) (`KismetMathLibrary.MakeVector` 0.0 CannonBarrelYLocation) false false))

(fn `SpawnProjectile`
  (bind _arrow (`self.Arrow`))
  (`|SpawnActorFromClass` "/Game/Blueprints/Actors/Projectiles/BP_Projectile.BP_Projectile_C" (`KismetMathLibrary.MakeTransform` (`SceneComponent.K2_GetComponentLocation` _arrow) (`SceneComponent.K2_GetComponentRotation` _arrow) (`KismetMathLibrary.Conv_DoubleToVector` (`self.ProjectileScale`))) "Undefined" "OverrideRootScale" null null))

(fn `UserConstructionScript`)